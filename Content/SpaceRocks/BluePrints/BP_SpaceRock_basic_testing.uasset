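; BP_SpaceRock_basic_testing is a basic test space rock actor that drifts, tumbles and bounces off what it hits.
; BeginPlay picks a random move vector within the GameState's spawn speed, plus a random spin.
; Tick applies both per frame, unswept and without delta-time scaling, until RootDestroyed is set.
; Hit approximates reflection by scaling each velocity axis by a factor from the hit normal via CalcBounce.
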(event EventTick
  (params (DeltaSeconds :type Float%20%28single-precision%29))
  ;[1 1 1] Move and Rotate Root Component (if rock is still in one piece)
  (if (not (Variables|Default|GetRootDestroyed))
    (Transformation|AddWorldOffset (Variables|Default|GetRootNode) (Variables|Default|GetRootMoveVector) false)
    (Class|Actor|AddActorWorldRotation (Variables|Default|GetRootRotation) false)))

(event EventBeginPlay
  ;[1 1 1] Set Up Initial Random Movement and Rotation (based on gamestate parameters)
  (bind _asspacerocksgamestate (Utilities|Casting|CastToSpaceRocksGameState (Game|GetGameState)))
  (bind _returnvalue (Class|SpaceRocksGameState|GetSpacerockSpawnSpeed _asspacerocksgamestate))
  (Variables|Default|SetMaxSpawnSpeed _returnvalue)
  (Variables|Default|SetMaxSpawnSpeed_neg (|0-x _returnvalue))
  (Variables|Default|SetRootMoveVector (Math|Vector|MakeVector (Math|Random|RandomFloatinRange (Variables|Default|GetMaxSpawnSpeed_neg) (Variables|Default|GetMaxSpawnSpeed)) (Math|Random|RandomFloatinRange (Variables|Default|GetMaxSpawnSpeed_neg) (Variables|Default|GetMaxSpawnSpeed)) (Math|Random|RandomFloatinRange (Variables|Default|GetMaxSpawnSpeed_neg) (Variables|Default|GetMaxSpawnSpeed))))
  (Variables|Default|SetRootRotation (Class|KismetMathLibrary|MakeRot (Math|Random|RandomFloatinRange -1.0 1.0) (Math|Random|RandomFloatinRange -1.0 1.0) (Math|Random|RandomFloatinRange -1.0 1.0))))

(event EventHit
  (params (MyComp :type Primitive%20Component%20Object%20Reference) (Other :type Actor%20Object%20Reference) (OtherComp :type Primitive%20Component%20Object%20Reference) (bSelfMoved :type Boolean) (HitLocation :type Vector :default "0, 0, 0") (HitNormal :type Vector :default "0, 0, 0") (NormalImpulse :type Vector :default "0, 0, 0") (Hit :type Hit%20Result%20Structure%20%28by%20ref%29))
  (bind (_x _y _z) (Math|Vector|BreakVector HitNormal))
  (bind _impactangleout (CallFunction|CalcBounce _x))
  (bind _impactangleout_2 (CallFunction|CalcBounce _y))
  (bind _impactangleout_3 (CallFunction|CalcBounce _z))
  (Variables|Default|SetImpactAngle (Math|Vector|MakeVector _impactangleout _impactangleout_2 _impactangleout_3))
  (Variables|Default|SetRootMoveVector (Math|Vector|MakeVector (|X*(0-Y) (.X (Math|Vector|BreakVector (Variables|Default|GetRootMoveVector))) (.X (Math|Vector|BreakVector (Variables|Default|GetImpactAngle)))) (|X*(0-Y) (.Y (Math|Vector|BreakVector (Variables|Default|GetRootMoveVector))) (.Y (Math|Vector|BreakVector (Variables|Default|GetImpactAngle)))) (|X*(0-Y) (.Z (Math|Vector|BreakVector (Variables|Default|GetRootMoveVector))) (.Z (Math|Vector|BreakVector (Variables|Default|GetImpactAngle)))))))

(fn ConstructionScript)

(fn CalcBounce
  (params (ImpactAngleIn :type Float%20%28single-precision%29))
  (bind _returnvalue (|x*2 ImpactAngleIn))
  (LocalVariables|Settemp _returnvalue)
  (if (< _returnvalue 0.0)
    (LocalVariables|Settemp (|0-x (LocalVariables|Gettemp))))
  (return (|x-1 (LocalVariables|Gettemp))))