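; Basic space rock actor that starts drifting and tumbling in a random direction when spawned.
; On BeginPlay it reads the spawn speed from SpaceRocksGameState and uses it as the symmetric bound for a random velocity on each axis.
; That vector is applied to RootNode as a velocity-change impulse, while RotatingMovement1 receives a small random rotation rate for the spin.
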(event EventBeginPlay
  ;[1 1 1] Set Up Initial Random Movement and Rotation (based on gamestate parameters)
  (bind _asspacerocksgamestate (Utilities|Casting|CastToSpaceRocksGameState (Game|GetGameState)))
  (bind _returnvalue (Class|SpaceRocksGameState|GetSpacerockSpawnSpeed _asspacerocksgamestate))
  (Variables|Default|SetMaxSpawnSpeed _returnvalue)
  (Variables|Default|SetMaxSpawnSpeed_neg (|0-x _returnvalue))
  (Variables|Default|SetRootMoveVector (Math|Vector|MakeVector (Math|Random|RandomFloatinRange (Variables|Default|GetMaxSpawnSpeed_neg) (Variables|Default|GetMaxSpawnSpeed)) (Math|Random|RandomFloatinRange (Variables|Default|GetMaxSpawnSpeed_neg) (Variables|Default|GetMaxSpawnSpeed)) (Math|Random|RandomFloatinRange (Variables|Default|GetMaxSpawnSpeed_neg) (Variables|Default|GetMaxSpawnSpeed))))
  (Variables|Default|SetRootRotation (Class|KismetMathLibrary|MakeRot (Math|Random|RandomFloatinRange -2e+01 2e+01) (Math|Random|RandomFloatinRange -2e+01 2e+01) (Math|Random|RandomFloatinRange -2e+01 2e+01)))
  (Physics|AddImpulse (Variables|Default|GetRootNode) (Variables|Default|GetRootMoveVector) "None" true)
  (Variables|/Script/Engine.RotatingMovementComponent|SetRotationRate (Variables|Default|GetRotatingMovement1) (Variables|Default|GetRootRotation)))

(fn ConstructionScript)